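; BP_DefaultGun is a hitscan gun that deals damage to BP_Character targets and triggers an attached perk.
; Fire line traces from the Trajectory component to a given end point, playing muzzle flash and sound on every shot and the player's HUD hit marker on character hits.
; ApplyDamage multiplies damage for head and neck bone hits, then executes the perk on the victim.
; BeginPlay adds a chain lightning component as that perk.
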(event EventBeginPlay
  (bind _returnvalue (AddComponent|AddBPChainLightningPerk))
  (Variables|Default|SetPerk _returnvalue))

(event Collision|EventActorBeginOverlap
  (params (OtherActor :type Actor%20Object%20Reference)))

(event EventTick
  (params (DeltaSeconds :type Float%20%28single-precision%29)))

(event EventFire
  (params (EndVector :type Vector :default "0, 0, 0"))
  ;[1 1 1] Firing
  (bind _outhit (Collision|LineTraceByChannel (Transformation|GetWorldLocation (Variables|Default|GetTrajectory)) EndVector "TraceTypeQuery1" false 0 "ForDuration"))
  (CallFunction|PlayEffects)
  (bind _asbp_character (Utilities|Casting|CastToBP_Character (.hitactor _outhit)))
  (CallFunction|PlayHUDAnims)
  (CallFunction|ApplyDamage _asbp_character (.hitbonename _outhit)))

(fn ConstructionScript)

(fn ApplyDamage
  (params (CharacterToDamage :type BP%20Character%20Object%20Reference) (BoneHit :type Name))
  (bind _perk (Variables|Default|GetPerk))
  (bind _damage (Variables|Default|GetDamage))
  (switch name BoneHit
    (:Default
      (LocalVariables|SetTotalDamage _damage))
    (:b_Neck
      (LocalVariables|SetTotalDamage (* _damage 1e+01) :!label _label))
    (:b_head
      (goto _label)))
  (Default|TakeDamage CharacterToDamage (LocalVariables|GetTotalDamage) BoneHit)
  (Utilities|IsValid (Utilities|ToObject(Interface) _perk)
    (:Is%20Valid
      (Default|ExecutePerk _perk (Utilities|Array|MakeArray CharacterToDamage)))))

(fn PlayEffects
  (bind _trajectory (Variables|Default|GetTrajectory))
  (bind _returnvalue (Transformation|GetWorldLocation _trajectory))
  (Effects|SpawnEmitteratLocation "/Game/StarterContent/Particles/MuzzleFlash.MuzzleFlash" _returnvalue "0, 0, 0" "0.400000,0.400000,0.400000")
  (Audio|PlaySoundatLocation "/Game/StarterContent/Audio/Explosion02.Explosion02" _returnvalue))

(fn PlayHUDAnims
  (bind _asbp_player_character (Utilities|Casting|CastToBP_PlayerCharacter (Game|GetPlayerCharacter 0)))
  (UserInterface|Animation|PlayAnimation (Variables|/Game/Characters/Blueprints/BP_PlayerCharacter.BP_PlayerCharacter_C|GetHUD _asbp_player_character) (Variables|/Game/HUD/BP_HUD.BP_HUD_C|GetHitMarkerFade (Variables|/Game/Characters/Blueprints/BP_PlayerCharacter.BP_PlayerCharacter_C|GetHUD _asbp_player_character)) 0.0 1 "Forward" 1.0))