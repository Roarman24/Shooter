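; Gun perk component that makes a hit arc lightning from the struck enemy through other nearby enemies.
; ExecutePerk takes the enemy from its params and base damage from the owning BP_DefaultGun, then loops to the closest not-yet-hit BP_Enemy within LightningRange.
; Each jump multiplies damage by DamageDecay, applies it and spawns a beam emitter between the two enemies.
; The chain ends when no valid target remains; EnemiesHit is never cleared here.
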(event EventBeginPlay)

(event EventTick
  (params (DeltaSeconds :type Float%20%28single-precision%29)))

(event EventExecutePerk
  (params (Params :type Array%20of%20Object%20Object%20References))
  (CallFunction|UnpackParams Params)
  (Variables|Default|SetIsChaining true)
  (CallFunction|ChainLightning))

(fn GetClosestEnemy
  (params (RootEnemy :type BP%20Enemy%20Object%20Reference) (EnemiesAlreadyHit :type Array%20of%20BP%20Enemy%20Object%20References))
  (LocalVariables|SetClosestDistance (Variables|Default|GetLightningRange))
  (bind _outactors (Actor|GetAllActorsOfClass "/Game/Characters/Blueprints/BP_Enemy.BP_Enemy_C"))
  (bind _available (CallFunction|RemoveAlreadyHitEnemies _outactors EnemiesAlreadyHit))
  (for _array_element _available
    (if (< (Transformation|GetDistanceTo _array_element RootEnemy) (LocalVariables|GetClosestDistance))
      (LocalVariables|SetClosestDistance (Transformation|GetDistanceTo _array_element RootEnemy))
      (LocalVariables|SetEnemyToChainTo _array_element)))
  (return (LocalVariables|GetEnemyToChainTo)))

(fn UnpackParams
  (params (Params :type Array%20of%20Object%20Object%20References))
  (bind _asbp_enemy (Utilities|Casting|CastToBP_Enemy (Utilities|Array|Get(acopy) Params)))
  (Variables|Default|SetCurrentEnemy _asbp_enemy)
  (bind _asbp_default_gun (Utilities|Casting|CastToBP_DefaultGun (Components|GetOwner)))
  (Variables|Default|SetBounceDamage (Variables|/Game/Guns/DefaultGun/BP_DefaultGun.BP_DefaultGun_C|GetDamage _asbp_default_gun)))

(fn CalculateBounceDamage
  (Variables|Default|SetBounceDamage (* (Variables|Default|GetBounceDamage) (Variables|Default|GetDamageDecay))))

(fn ChainLightning
  (Utilities|Array|Add (LocalVariables|GetEnemiesHit) (Variables|Default|GetCurrentEnemy))
  (while (Variables|Default|GetIsChaining)
    (bind _closestenemy (CallFunction|GetClosestEnemy (Variables|Default|GetCurrentEnemy) (LocalVariables|GetEnemiesHit)))
    (if (Utilities|IsValid _closestenemy)
      (CallFunction|CalculateBounceDamage)
      (CallFunction|SpawnLightningEffect (Variables|Default|GetCurrentEnemy) _closestenemy)
      (Default|TakeDamage _closestenemy (Variables|Default|GetBounceDamage) "None")
      (Variables|Default|SetCurrentEnemy _closestenemy)
      (Utilities|Array|Add (LocalVariables|GetEnemiesHit) (Variables|Default|GetCurrentEnemy))
      (else
        (Variables|Default|SetIsChaining false)))))

(fn RemoveAlreadyHitEnemies
  (params (FoundEnemies :type Array%20of%20BP%20Enemy%20Object%20References) (AlreadyHitEnemies :type Array%20of%20BP%20Enemy%20Object%20References))
  (for _array_element FoundEnemies
    (if (not (Utilities|Array|ContainsItem AlreadyHitEnemies _array_element))
      (Utilities|Array|Add (LocalVariables|GetAvailableEnemies) _array_element)))
  (return (LocalVariables|GetAvailableEnemies)))

(fn SpawnLightningEffect
  (params (RootEnemy :type BP%20Enemy%20Object%20Reference) (NextEnemy :type BP%20Enemy%20Object%20Reference))
  (bind _returnvalue (Transformation|GetActorTransform RootEnemy))
  (bind _returnvalue_2 (Effects|SpawnEmitteratLocation "/Game/MyParticleSystems/Beam/P_Beam.P_Beam" (.location _returnvalue) (.rotation _returnvalue)))
  (Class|ParticleSystemComponent|SetBeamSourcePoint _returnvalue_2 0 (.location _returnvalue))
  (Class|ParticleSystemComponent|SetBeamTargetPoint _returnvalue_2 0 (Transformation|GetActorLocation NextEnemy)))