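; BP_Character is a character Blueprint with basic health, damage and death handling, and it caches the BP_GameManager on BeginPlay.
; TakeDamage stores the hit bone, subtracts and prints Health, then calls CheckHealth, which triggers Die below 1.
; CheckDeathType maps head and neck hits to a specific death enum value and passes it to Die, whose body here only destroys the actor.
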(event EventBeginPlay
  (bind _outactors (Actor|GetAllActorsOfClass "/Game/GameModes/BP_GameManager.BP_GameManager_C"))
  (Variables|Default|SetGameManager (Utilities|Array|Get(acopy) _outactors)))

(event Collision|EventActorBeginOverlap
  (params (OtherActor :type Actor%20Object%20Reference)))

(event EventTick
  (params (DeltaSeconds :type Float%20%28single-precision%29)))

(event EventCheckHealth
  ;[1 1 1] Default Character Health functionality
  (if (< (Variables|Default|GetHealth) 1.0)
    (bind _deathtype (CallFunction|CheckDeathType))
    (CallFunction|Die _deathtype)))

(event EventTakeDamage
  (params (DamageToTake :type Float%20%28single-precision%29) (LastBoneHit :type Name :default "None"))
  ;[1 1 1] Default Character Health functionality
  (Variables|Default|SetLastBoneHit LastBoneHit)
  (bind _output_get (Variables|Default|SetHealth (- (Variables|Default|GetHealth) DamageToTake)))
  (Development|PrintString (Utilities|String|ToString(Float) _output_get))
  (CallFunction|CheckHealth))

(event EventDie
  (params (DeathType :type E_DeathType%20Enum :default "NewEnumerator0"))
  ;[1 1 1] Default Character Health functionality
  (Actor|DestroyActor))

(fn ConstructionScript)

(fn CheckDeathType
  (switch name (Variables|Default|GetLastBoneHit)
    (:Default
      _)
    (:b_head
      (LocalVariables|SetDeath "NewEnumerator2" :!label _label))
    (:b_Neck
      (goto _label)))
  (return (LocalVariables|GetDeath)))