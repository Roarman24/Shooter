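; BP_Enemy is an enemy that damages the player on contact and awards points when it dies.
; When a player character enters its DamageRange, it applies damage, spawns an explosion and destroys itself, without going through Die or awarding points.
; The overridden Die event passes the death type and the enemy's Worth to the GameManager through SendPointsToGameManager, then destroys the actor.
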(event OnComponentBeginOverlap(DamageRange)
  (params (OverlappedComponent :type Primitive%20Component%20Object%20Reference) (OtherActor :type Actor%20Object%20Reference) (OtherComp :type Primitive%20Component%20Object%20Reference) (OtherBodyIndex :type Integer) (bFromSweep :type Boolean) (SweepResult :type Hit%20Result%20Structure%20%28by%20ref%29))
  ;[1 1 1] Damage to Player
  (bind _asbp_player_character (Utilities|Casting|CastToBP_PlayerCharacter OtherActor))
  (Default|TakeDamage _asbp_player_character (Variables|Default|GetDamage) "None")
  (Effects|SpawnEmitteratLocation "/Game/StarterContent/Particles/P_Explosion.P_Explosion" (.location (Transformation|GetActorTransform)))
  (Actor|DestroyActor))

(event EventBeginPlay)

(event Collision|EventActorBeginOverlap
  (params (OtherActor :type Actor%20Object%20Reference)))

(event EventTick
  (params (DeltaSeconds :type Float%20%28single-precision%29)))

(event EventDie
  (params (DeathType :type E_DeathType%20Enum :default "NewEnumerator0"))
  ;[1 1 1] Override Death to award player points
  (CallFunction|SendPointstoGameManager DeathType)
  (Actor|DestroyActor))

(fn ConstructionScript)

(fn SendPointstoGameManager
  (params (DeathType :type E_DeathType%20Enum :default "NewEnumerator0"))
  (Default|AwardPoints (Variables|Default|GetGameManager) DeathType (Variables|Default|GetWorth)))