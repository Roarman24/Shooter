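; BP_GameManager is a scoring manager that awards points for kills reported by death type.
; AwardPoints passes the base points through for a normal kill, or multiplies them by HeadshotBonus for a headshot kill.
; SetPoints then adds the result to both TotalPoints and AvailablePoints; nothing in this file deducts from either.
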(event Custom|AwardPoints
  (params (DeathType :type E_DeathType%20Enum :default "NewEnumerator0") (Points :type Integer))
  (switch Utilities|FlowControl|Switch|SwitchonE_DeathType DeathType
    (:NewEnumerator0
      (Variables|Default|SetTotalPointsToAward Points))
    (:NewEnumerator2
      (Variables|Default|SetTotalPointsToAward (* Points (Variables|Default|GetHeadshotBonus)))))
  (CallFunction|SetPoints (Variables|Default|GetTotalPointsToAward)))

(event EventBeginPlay)

(event Collision|EventActorBeginOverlap
  (params (OtherActor :type Actor%20Object%20Reference)))

(event EventTick
  (params (DeltaSeconds :type Float%20%28single-precision%29)))

(fn ConstructionScript)

(fn SetPoints
  (params (PointsToAdd :type Integer))
  (Variables|Default|SetTotalPoints (+ (Variables|Default|GetTotalPoints) PointsToAdd))
  (Variables|Default|SetAvailablePoints (+ (Variables|Default|GetAvailablePoints) PointsToAdd)))